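; AI controller for a vision-driven vehicle pawn that analyses a camera feed to locate the end of the track.
; On BeginPlay it caches the pawn's vehicle movement component and applies full throttle.
; While DoUpdates is set, Tick runs MovementUpdate, which derives distance and direction from InitialPoint to the FindTrackEnd result.
; Tick does not use those outputs, so no steering is applied here.
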(event EventBeginPlay
  (bind _output_get (Variables|Default|SetVehiclePawn (.AsVision%20Vehicles%20Pawn%20Blueprint (Utilities|Casting|CastToVisionVehiclesPawn_Blueprint (Pawn|GetControlledPawn)))))
  (Variables|Default|SetVehicleMovementComponent (Variables|/Script/PhysXVehicles.WheeledVehicle|GetVehicleMovement _output_get))
  (Class|WheeledVehicleMovementComponent|SetThrottleInput (Variables|Default|GetVehicleMovementComponent) 1.0))

(event EventTick
  (params (DeltaSeconds :type Float%20%28single-precision%29))
  (if (Variables|Default|GetDoUpdates)
    (CallFunction|MovementUpdate)))

(fn ConstructionScript)

(fn MovementUpdate
  (bind _returnvalue (Class|VisionVehiclesAIController|FindTrackEnd (Variables|Default|GetCameraFeed) 4 4))
  (return (Math|Vector2D|Vector2DLength (- _returnvalue (Variables|Default|GetInitialPoint))) (Math|Vector2D|Normalize2D (- _returnvalue (Variables|Default|GetInitialPoint)))))