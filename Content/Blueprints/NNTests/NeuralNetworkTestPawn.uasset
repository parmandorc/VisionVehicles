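; Test pawn that exercises a neural network by training it online on randomly generated data.
; BeginPlay gets the network instance and initializes its layer and learning-rate settings.
; Each Tick runs the network on random inputs, trains it against targets from ProcessFunction, then prints inputs, outputs, targets and error.
; ProcessFunction is an empty stub here, so this class defines no real target function.
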(event EventBeginPlay
  (bind _returnvalue (Class|NeuralNetwork|GetInstance))
  (bind _output_get (Variables|Default|SetNeuralNetwork _returnvalue))
  (Class|NeuralNetwork|Init _output_get (Variables|Default|GetInputs) (Variables|Default|GetOutputs) (Variables|Default|GetHidden%20Layers) (Variables|Default|GetLearning%20Rate) (Variables|Default|GetLearning%20Rate%20Decay)))

(event Collision|EventActorBeginOverlap
  (params (OtherActor :type Actor%20Object%20Reference)))

(event EventTick
  (params (DeltaSeconds :type Float%20%28single-precision%29))
  (bind _neuralnetwork (Variables|Default|GetNeuralNetwork))
  (bind _inputs_array (CallFunction|CreateInputs))
  (bind _returnvalue (Class|NeuralNetwork|Run _neuralnetwork _inputs_array))
  (bind _outputs (CallFunction|ProcessInputs _inputs_array))
  (bind _returnvalue_2 (Class|NeuralNetwork|Train _neuralnetwork _inputs_array _outputs))
  (bind _string (CallFunction|ToString _inputs_array _returnvalue _outputs _returnvalue_2))
  (Development|PrintString _string))

(fn ConstructionScript)

(fn CreateInputs
  (Utilities|Array|Clear (LocalVariables|GetInputsArray))
  (for _index (range 0 (- (Variables|Default|GetInputs) 1))
    (Utilities|Array|Add (LocalVariables|GetInputsArray) (Math|Random|RandomFloatinRange 0.0 1.0)))
  (return (LocalVariables|GetInputsArray)))

(fn ProcessInputs
  (params (Inputs :type Array%20of%20Floats%20%28single-precision%29))
  (Utilities|Array|Clear (LocalVariables|GetProcessedOutputs))
  (for _index (range 0 (- (Variables|Default|GetOutputs) 1))
    (Utilities|Array|Add (LocalVariables|GetProcessedOutputs) (Utilities|ProcessFunction Inputs _index)))
  (return (LocalVariables|GetProcessedOutputs)))

(fn ToString
  (params (Inputs :type Array%20of%20Floats%20%28single-precision%29) (Outputs :type Array%20of%20Floats%20%28single-precision%29) (Expected%20Outpus :type Array%20of%20Floats%20%28single-precision%29) (Error :type Float%20%28single-precision%29))
  (Utilities|FlowControl|Sequence
    (:then_0
      (LocalVariables|SetResult%20String "Inputs:"))
    (:then_1
      (for _array_element Inputs
        (LocalVariables|SetResult%20String (Utilities|String|Append (LocalVariables|GetResult%20String) " " (Utilities|String|ToString(Float) _array_element)))))
    (:then_2
      (LocalVariables|SetResult%20String (Utilities|String|Append (LocalVariables|GetResult%20String) ", Outputs:")))
    (:then_3
      (for _array_element_2 Outputs
        (LocalVariables|SetResult%20String (Utilities|String|Append (LocalVariables|GetResult%20String) " " (Utilities|String|ToString(Float) _array_element_2)))))
    (:then_4
      (LocalVariables|SetResult%20String (Utilities|String|Append (LocalVariables|GetResult%20String) ", Expected:")))
    (:then_5
      (for _array_element_3 Expected%20Outpus
        (LocalVariables|SetResult%20String (Utilities|String|Append (LocalVariables|GetResult%20String) " " (Utilities|String|ToString(Float) _array_element_3)))))
    (:then_6
      (LocalVariables|SetResult%20String (Utilities|String|Append (LocalVariables|GetResult%20String) ", Error: " (Utilities|String|ToString(Float) Error))))
    (:then_7
      (return (LocalVariables|GetResult%20String)))))