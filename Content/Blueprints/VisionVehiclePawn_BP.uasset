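; Vehicle pawn that learns to drive from the player's input through a neural network, then drives itself.
; Each tick it reduces the vision component's camera feed to a track-end pixel difference, the network's sole input.
; In learning mode it stores that with steering, throttle and handbrake, training on random samples from a capped replay memory.
; A key toggles autonomous mode, where network outputs drive the vehicle; a widget displays the network.
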(event EventBeginPlay
  (bind _seconds (Class|GameplayStatics|GetAccurateRealTime))
  (Utilities|FlowControl|Sequence
    (:then_0
      (Math|Random|SetRandomStreamSeed (Math|Random|MakeRandomStream _seconds) _seconds))
    (:then_1
      (bind _returnvalue (UserInterface|CreateWidget "/Game/Blueprints/NeuralNetworkUI.NeuralNetworkUI_C" (Game|GetPlayerController 0)))
      (UserInterface|Viewport|AddtoViewport _returnvalue 0)
      (Variables|Default|SetUI _returnvalue))))

(event EventTick
  (params (DeltaSeconds :type Float%20%28single-precision%29))
  (bind _ui (Variables|Default|GetUI))
  (Utilities|FlowControl|Sequence
    (:then_0
      (CallFunction|AnalyzeCameraFeed))
    (:then_1
      (CallFunction|InteractwithNeuralNetwork))
    (:then_2
      (if (not (Variables|/Game/Blueprints/NeuralNetworkUI.NeuralNetworkUI_C|GetDrawNetwork _ui))
        (Default|SetUpDrawingParameters _ui)
        (Variables|/Game/Blueprints/NeuralNetworkUI.NeuralNetworkUI_C|SetDrawNetwork _ui true)))))

(event Input|ActionEvents|InputActionHandbrake
  (params (Key :type Key%20Structure :default "AnyKey"))
  (bind _vehiclemovement (Variables|Default|GetVehicleMovement))
  (bind _operationmode (Variables|Default|GetOperationMode))
  (bind _returnvalue (Utilities|Enum|Equal(Enum) "NewEnumerator0" _operationmode))
  ;[1 1 1] Handbrake input
  (:Pressed
    (if _returnvalue
      (bind _output_get (Variables|Useroutputs|SetHandbrakeOutput true))
      (Class|WheeledVehicleMovementComponent|SetHandbrakeInput _vehiclemovement _output_get)))
  (:Released
    (if _returnvalue
      (bind _output_get_2 (Variables|Useroutputs|SetHandbrakeOutput false))
      (Class|WheeledVehicleMovementComponent|SetHandbrakeInput _vehiclemovement _output_get_2))))

(event Input|ActionEvents|InputActionSwitchControlMode
  (params (Key :type Key%20Structure :default "AnyKey"))
  ;[1 1 1] Switch operation mode
  (:Pressed
    (switch Utilities|FlowControl|Switch|SwitchonCarOperationMode (Variables|Default|GetOperationMode)
      (:NewEnumerator0
        (Variables|Default|SetOperationMode "NewEnumerator1")
        (Class|WheeledVehicleMovementComponent|SetThrottleInput (Variables|Default|GetVehicleMovement) 1.0))
      (:NewEnumerator1
        (Variables|Default|SetOperationMode "NewEnumerator0")))))

(event Input|AxisEvents|InputAxisMoveForward
  (params (AxisValue :type Float%20%28single-precision%29))
  ;[1 1 1] Throttle input
  (if (Utilities|Enum|Equal(Enum) "NewEnumerator0" (Variables|Default|GetOperationMode))
    (bind _output_get (Variables|Useroutputs|SetThrottleOutput AxisValue))
    (Class|WheeledVehicleMovementComponent|SetThrottleInput (Variables|Default|GetVehicleMovement) _output_get)))

(event Input|AxisEvents|InputAxisMoveRight
  (params (AxisValue :type Float%20%28single-precision%29))
  ;[1 1 1] Steering input
  (if (Utilities|Enum|Equal(Enum) "NewEnumerator0" (Variables|Default|GetOperationMode))
    (bind _output_get (Variables|Useroutputs|SetSteeringOutput AxisValue))
    (Class|WheeledVehicleMovementComponent|SetSteeringInput (Variables|Default|GetVehicleMovement) _output_get)))

(fn ConstructionScript)

(fn AnalyzeCameraFeed
  (bind _returnvalue (Class|VehicleVisionComponent|GetCameraFeed (Variables|Default|GetVisionComponent)))
  (bind _output_get (Variables|Default|SetCameraFeed _returnvalue))
  (if (> (Utilities|Array|Length _output_get) 0)
    (bind _returnvalue_2 (Class|VisionVehiclesPawn|FindTrackEnd _output_get))
    (Variables|Default|SetPixelsDifferenceInput (- (.x _returnvalue_2) (.y _returnvalue_2)))
    (else
      (Development|PrintString "Ananyze camera feed: camera feed is empty."))))

(fn ControlCarUsingInputs
  (params (Inputs :type Array%20of%20Floats%20%28single-precision%29))
  (if (== (LocalVariables|GetRequiredInputsNumber) (Utilities|Array|Length Inputs))
    (Utilities|FlowControl|Sequence
      (:then_0
        (Class|WheeledVehicleMovementComponent|SetSteeringInput (Variables|Default|GetVehicleMovement) (Utilities|Array|Get(acopy) Inputs)))
      (:then_1
        (Class|WheeledVehicleMovementComponent|SetThrottleInput (Variables|Default|GetVehicleMovement) (Utilities|Array|Get(acopy) Inputs 1)))
      (:then_2
        (Class|WheeledVehicleMovementComponent|SetHandbrakeInput (Variables|Default|GetVehicleMovement) (Math|Conversions|ToBoolean(Integer) (Math|Integer|%(Integer) (Math|Float|Truncate (Utilities|Array|Get(acopy) Inputs 2)) 2)))))))

(fn InteractwithNeuralNetwork
  (bind (_result _index) (Utilities|GetRandomElementfromMemory))
  (LocalVariables|SetInputs (Utilities|Array|MakeArray (Variables|Default|GetPixelsDifferenceInput)))
  (switch Utilities|FlowControl|Switch|SwitchonCarOperationMode (Variables|Default|GetOperationMode)
    (:NewEnumerator0
      ;[1 1 1] Add input to the memory
      (bind _returnvalue (Utilities|Array|Add (Variables|Default|GetStoredMemory) (Utilities|Struct|MakeInputsMemory (LocalVariables|GetInputs) (Utilities|Array|MakeArray (Variables|Useroutputs|GetSteeringOutput) (Variables|Useroutputs|GetThrottleOutput) (Math|Conversions|ToFloat(Boolean) (Variables|Useroutputs|GetHandbrakeOutput))))))
      (if (> _returnvalue (Variables|Default|GetInputsMemorySize))
        (Class|VisionVehiclesPawn|TrainNetwork (.inputs _result) (.outputs _result))
        (Utilities|Array|RemoveIndex (Variables|Default|GetStoredMemory) _index)))
    (:NewEnumerator1
      (bind _returnvalue_2 (Class|VisionVehiclesPawn|RunNetwork (LocalVariables|GetInputs)))
      (CallFunction|ControlCarUsingInputs _returnvalue_2))))