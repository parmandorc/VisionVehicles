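; AI controller for a VisionVehiclesPawn that aims to read the track from a camera feed.
; On BeginPlay it caches the pawn's vehicle movement component and sets full throttle.
; While DoUpdates is set, each Tick runs MovementUpdate, which locates the track end in the feed and derives distance and direction from InitialPoint.
; Tick discards those results, so no steering or throttle correction is applied.
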(event EventBeginPlay
  (bind _asvision_vehicles_pawn (Utilities|Casting|CastToVisionVehiclesPawn (Pawn|GetControlledPawn)))
  (Variables|Default|SetVehicleMovementComponent (Variables|/Script/PhysXVehicles.WheeledVehicle|GetVehicleMovement _asvision_vehicles_pawn))
  (Class|WheeledVehicleMovementComponent|SetThrottleInput (Variables|Default|GetVehicleMovementComponent) 1.0))

(event EventTick
  (params (DeltaSeconds :type Float%20%28single-precision%29))
  (if (Variables|Default|GetDoUpdates)
    (CallFunction|MovementUpdate)))

(fn ConstructionScript)

(fn MovementUpdate
  (bind _returnvalue (Class|VisionVehiclesAIController|FindTrackEnd (Variables|Default|GetCameraFeed) 4 4))
  (return (Math|Vector2D|Vector2DLength (- _returnvalue (Variables|Default|GetInitialPoint))) (Math|Vector2D|Normalize2D (- _returnvalue (Variables|Default|GetInitialPoint)))))